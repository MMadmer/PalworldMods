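; BP_MeshAnalizer is an actor that enables Render CustomDepth on mesh components of supplied actors, spreading the work across several ticks.
; SetCachedActors divides the list by IterationsCount into a per-tick batch, with the remainder handed out one extra actor per tick.
; StartAnalize turns on Tick, which processes and removes each batch, skipping invalid actors and blacklisted classes.
; An empty queue disables Tick, clears the busy flag behind GetCanAnalize and fires OnAnalizeDone.
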(event Custom|StartAnalize
  (Variables|Default|SetInProcess true)
  (Actor|Tick|SetActorTickEnabled true))

(event EventTick
  (params (DeltaSeconds :type Float%20%28single-precision%29))
  (if (Utilities|Array|IsNotEmpty (Variables|Default|GetCachedActors))
    (CallFunction|TickIteration)
    (else
      (Actor|Tick|SetActorTickEnabled false)
      (Variables|Default|SetInProcess false)
      (Default|CallOnAnalizeDone))))

(fn ConstructionScript)

(fn SetCachedActors
  (params (Actors :type Array%20of%20Actor%20Object%20References))
  (bind _output_get (Variables|Default|SetCachedActors Actors))
  (Variables|Default|SetBonusActors (Math|Float|Truncate (.Remainder (Math|Float|Division(WholeandRemainder) (Math|Conversions|ToFloat(Integer) (Utilities|Array|Length _output_get)) (Math|Conversions|ToFloat(Integer) (Variables|AnalizeSettings|GetIterationsCount))))))
  (Variables|Default|SetActorsPerTick (.ReturnValue (Math|Float|Division(WholeandRemainder) (Math|Conversions|ToFloat(Integer) (Utilities|Array|Length _output_get)) (Math|Conversions|ToFloat(Integer) (Variables|AnalizeSettings|GetIterationsCount))))))

(fn TickIteration
  (bind _cachedactors (Variables|Default|GetCachedActors))
  (bind _bonusactors (Variables|Default|GetBonusActors))
  (LocalVariables|SetCurrentActors (+ (Variables|Default|GetActorsPerTick) (Math|Conversions|ToInteger(Boolean) (Math|Conversions|ToBoolean(Integer) (Variables|Default|GetBonusActors)))))
  (for (_array_element _array_index) (Variables|Default|GetCachedActors)
    (if (< _array_index (LocalVariables|GetCurrentActors))
      (Utilities|IsValid _array_element
        (:Is%20Valid
          (if (< (Utilities|Array|FindItem (Variables|Default|GetClassBlackList) (Utilities|GetClass _array_element)) 0)
            (for _array_element_2 (Actor|GetComponentsByClass _array_element "/Script/Engine.MeshComponent")
              (Rendering|SetRenderCustomDepth _array_element_2 true)))))))
  (Utilities|FlowControl|ForLoopwithBreak 0 (- (LocalVariables|GetCurrentActors) 1) :!label _label
    (:LoopBody
      (if (Utilities|Array|IsValidIndex _cachedactors)
        (Utilities|Array|RemoveIndex _cachedactors)
        (else
          (goto _label Break))))
    (:Completed
      (if (> _bonusactors 0)
        (Math|Integer|DecrementInt _bonusactors)))))

(fn GetCanAnalize
  (return (not (Variables|Default|GetInProcess))))