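; Actor component for a Palworld character that plays "gachi" voice clips in reaction to gameplay events.
; It finds the owner's "gachi"-tagged AudioComponent, then binds movement, stamina, status, damage, death and action delegates, plus a delayed player-only greeting.
; Damage relative to max HP picks a random tiered clip, jumps and landings roll a chance, and actions resolve through an inverted ActionMap.
; PlaySound sets attenuation by loudness level on that single AudioComponent.
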(event Custom|OnJump
  (params (Component :type Pal%20Character%20Movement%20Component%20Object%20Reference))
  (Utilities|CanPlay (Variables|Chances|GetOnJumpChance)
    (:True
      (CallFunction|PlaySound (Variables|Default|GetGachiSound) "/Game/Mods/GachiWorld_P/Sounds/Man/Jump_Agh.Jump_Agh" "NewEnumerator0"))))

(event Custom|OnLand
  (params (Component :type Pal%20Character%20Movement%20Component%20Object%20Reference) (Hit :type Hit%20Result%20Structure%20%28by%20ref%29))
  (Utilities|CanPlay (Variables|Chances|GetOnLandChance)
    (:True
      (CallFunction|PlaySound (Variables|Default|GetGachiSound) "/Game/Mods/GachiWorld_P/Sounds/Man/Land_Ohh.Land_Ohh" "NewEnumerator0"))))

(event Custom|OnStaminaOver
  (CallFunction|PlaySound (Variables|Default|GetGachiSound) "/Game/Mods/GachiWorld_P/Sounds/Man/PlayerOnly/StaminaOver_Yeeeeeeah.StaminaOver_Yeeeeeeah" "NewEnumerator1"))

(event Custom|OnPlayerStart
  (if (Class|GameplayStatics|ObjectIsA (Variables|Default|GetOwner) "/Script/Pal.PalPlayerCharacter")
    (CallFunction|PlaySound (Variables|Default|GetGachiSound) "/Game/Mods/GachiWorld_P/Sounds/Man/PlayerOnly/Start_welcome-to-the-club.Start_welcome-to-the-club" "NewEnumerator0")))

(event EventBeginPlay
  (Components|Tick|SetComponentTickEnabled false)
  (bind _aspal_character (Utilities|Casting|CastToPalCharacter (Components|GetOwner)))
  (bind _output_get (Variables|Default|SetOwner _aspal_character))
  (bind _array_element (Utilities|Array|ForEachLoopwithBreak (Actor|GetComponentsbyTag _output_get "/Script/Engine.AudioComponent" "gachi") :!label _label)
    (:LoopBody
      (Variables|Default|SetGachiSound _array_element)
      (goto _label Break))
    (:Completed
      (Utilities|IsValid (Variables|Default|GetGachiSound)
        (:Is%20Valid
          (Utilities|Time|SetTimerbyEvent (delegate Custom|OnPlayerStart) 1.0 false 1.0)
          (EventDispatchers|AssignOnJumpDelegate (Class|PalCharacter|GetPalCharacterMovementComponent (Variables|Default|GetOwner)) (delegate Custom|OnJump))
          (EventDispatchers|AssignOnLandedDelegate (Class|PalCharacter|GetPalCharacterMovementComponent (Variables|Default|GetOwner)) (delegate Custom|OnLand))
          (EventDispatchers|AssignOnSPOverheatDelegate (Variables|/Script/Pal.PalCharacter|GetCharacterParameterComponent (Variables|Default|GetOwner)) (delegate Custom|OnStaminaOver))
          (CallFunction|AssignonStatuses)
          (CallFunction|AssignonDamage)
          (CallFunction|AssignAction))))))

(event Custom|AssignOnStatuses
  (EventDispatchers|AssignOnAddStatus (Variables|/Script/Pal.PalCharacter|GetStatusComponent (Variables|Default|GetOwner)) (delegate Custom|OnAddStatus)))

(event Custom|OnAddStatus
  (params (StatusComponent :type Pal%20Status%20Component%20Object%20Reference) (StatusId :type EPalStatusID%20Enum :default "None") (Status :type Pal%20Status%20Base%20Object%20Reference))
  (switch Utilities|FlowControl|Switch|SwitchonEPalStatusID StatusId
    (:Happiness
      (CallFunction|OnHappy))
    (:LavaDamage
      (CallFunction|OnBurn :!label _label))
    (:Burn
      (goto _label))))

(event Custom|OnBurn
  (CallFunction|PlaySound (Variables|Default|GetGachiSound) "/Game/Mods/GachiWorld_P/Sounds/Man/Burn_AAAAA.Burn_AAAAA" "NewEnumerator2"))

(event Custom|OnHappy
  (CallFunction|PlaySound (Variables|Default|GetGachiSound) "/Game/Mods/GachiWorld_P/Sounds/Man/Eat_mmmm.Eat_mmmm" "NewEnumerator0"))

(event Custom|AssignOnDamage
  (bind _owner (Variables|Default|GetOwner))
  (bind _damagereactioncomponent (Variables|/Script/Pal.PalCharacter|GetDamageReactionComponent _owner))
  (EventDispatchers|AssignOnDamageDelegateAlways _damagereactioncomponent (delegate Custom|OnTakeAnyDamage))
  (EventDispatchers|AssignOnDeadDelegate _damagereactioncomponent (delegate Custom|OnDead)))

(event Custom|OnLittleDamage
  (CallFunction|PlaySound (Variables|Default|GetGachiSound) (.OutItem (Utilities|Array|Random (Variables|OnDamage|GetLittleDamage))) "NewEnumerator1"))

(event Custom|OnMiddleDamage
  (CallFunction|PlaySound (Variables|Default|GetGachiSound) (.OutItem (Utilities|Array|Random (Variables|OnDamage|GetMiddleDamage))) "NewEnumerator1"))

(event Custom|OnTakeAnyDamage
  (params (DamageResult :type Pal%20Damage%20Result%20Structure))
  (bind _output_get (Variables|OnDamage|SetDamageBuffer (Math|Float|MapRangeClamped (Math|Conversions|ToFloat(Integer) (.damage DamageResult)) 0.0 (Class|FixedPoint64MathLibrary|ConvertFixedPoint64toFloat (Class|PalCharacterParameterComponent|GetMaxHP (Variables|/Script/Pal.PalCharacter|GetCharacterParameterComponent (Variables|Default|GetOwner)))) 0.0 1.0)))
  (if (> _output_get (Variables|OnDamage|GetNormDamage))
    (CallFunction|OnBigDamage)
    (elif (> (Variables|OnDamage|GetDamageBuffer) (Variables|OnDamage|GetMinDamage))
      (CallFunction|OnMiddleDamage)
      (else
        (CallFunction|OnLittleDamage)))))

(event Custom|OnDead
  (params (DeadInfo :type Pal%20Dead%20Info%20Structure))
  (CallFunction|PlaySound (Variables|Default|GetGachiSound) "/Game/Mods/GachiWorld_P/Sounds/Man/Dead_Haaaaa.Dead_Haaaaa" "NewEnumerator2"))

(event Custom|OnBigDamage
  (CallFunction|PlaySound (Variables|Default|GetGachiSound) (.OutItem (Utilities|Array|Random (Variables|OnDamage|GetBigDamage))) "NewEnumerator1"))

(event Custom|AssignAction
  (Utilities|SwapActionMap
    (:Output
      (EventDispatchers|AssignOnActionBeginDelegate (Variables|/Script/Pal.PalCharacter|GetActionComponent (Variables|Default|GetOwner)) (delegate Custom|OnActionBegin)))))

(event Custom|OnActionBegin
  (params (action :type Pal%20Action%20Base%20Object%20Reference))
  (bind _returnvalue (Utilities|GetClass action))
  (bind _actions (Variables|OnAction|GetActions))
  (bind _value (Utilities|Map|Find _actions _returnvalue))
  (CallFunction|LuaPrint (Utilities|String|Append "[GachiWorld] " (Utilities|String|EnumtoString _value)))
  (switch Utilities|FlowControl|Switch|SwitchonEPalActionType _value
    (:None
      (Utilities|Casting|CastToPalAction_SleepPlayerBed action)
      (Actions|OnSleep))
    (:Sleep
      (Actions|OnSleep))
    (:Eat
      (Actions|OnEat))
    (:Stan
      (Actions|OnStun))))

(fn PlaySound
  (params (AudioComponent :type Audio%20Component%20Object%20Reference%20%28by%20ref%29) (Sound :type Sound%20Base%20Object%20Reference) (AudioLevel :type E_AudioLevels%20Enum :default "NewEnumerator0"))
  (Variables|/Script/Engine.AudioComponent|SetAttenuationSettings AudioComponent (Utilities|Select :Index AudioLevel :NewEnumerator0 "/Game/Mods/GachiWorld_P/Sounds/AudioSettings/MS_Quiet.MS_Quiet" :NewEnumerator1 "/Game/Mods/GachiWorld_P/Sounds/AudioSettings/MS_Normal.MS_Normal" :NewEnumerator2 "/Game/Mods/GachiWorld_P/Sounds/AudioSettings/MS_Loud.MS_Loud" :NewEnumerator3 "/Game/Mods/GachiWorld_P/Sounds/AudioSettings/MS_Far.MS_Far"))
  (Audio|Components|Audio|SetSound AudioComponent Sound)
  (Audio|Components|Audio|Play AudioComponent 0.0))

(fn OnEat
  (CallFunction|PlaySound (Variables|Default|GetGachiSound) "/Game/Mods/GachiWorld_P/Sounds/Man/Eat_mmmm.Eat_mmmm" "NewEnumerator0"))

(fn OnStun
  (CallFunction|PlaySound (Variables|Default|GetGachiSound) "/Game/Mods/GachiWorld_P/Sounds/Man/Stun_Do_you_like_watch_on_me.Stun_Do_you_like_watch_on_me" "NewEnumerator1"))

(fn OnSleep
  (CallFunction|PlaySound (Variables|Default|GetGachiSound) "/Game/Mods/GachiWorld_P/Sounds/Man/PlayerOnly/Sleep_Agh_Oh.Sleep_Agh_Oh" "NewEnumerator1"))